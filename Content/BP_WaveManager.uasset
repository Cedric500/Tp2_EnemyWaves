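; BP_WaveManager runs enemy waves, stepping through WaveNumberArray from BeginPlay.
; Each wave calls Spawnable with EnemyForWaves on one ranged and one base enemy spawner, both found by class.
; After a short delay it checks EnemiesAlive once; at zero it raises the enemy count and manually advances the loop.
; Nothing here repeats that check, so waves halt if enemies remain.
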(event EventBeginPlay
  (Utilities|ManualforEachLoop (Variables|Default|GetWave%20number%20%28Array%29) :!label _label
    (:Loop%20Body
      (bind _returnvalue (Actor|GetActorOfClass "/Game/BP_BaseEnemySpawner.BP_BaseEnemySpawner_C"))
      (bind _returnvalue_2 (Actor|GetActorOfClass "/Game/BP_RangeEnemySpawner.BP_RangeEnemySpawner_C"))
      (Default|Spawnable _returnvalue_2 (Variables|Default|GetEnemy%20for%20waves))
      (Utilities|FlowControl|Delay 2.0)
      (if (== (Variables|Default|GetEnemies%20alive) 0)
        (Variables|Default|SetEnemy%20for%20waves (+ (Variables|Default|GetEnemy%20for%20waves) 3))
        (goto _label Next)))))

(fn ConstructionScript)