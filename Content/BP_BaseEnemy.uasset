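; Base enemy pawn that chases the player, deals damage on contact and reports its death to the wave manager.
; Tick issues AI MoveTo toward the first-person character, and capsule overlaps send damage through BPI_Damageable.
; TakeDamage lowers HP and, at zero, decrements EnemiesAlive, notifies BP_WaveManager, increments the player's kill count and destroys the actor.
; GetNuked kills instantly with the same notifications, but does not decrement EnemiesAlive itself.
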(event OnComponentBeginOverlap(CapsuleComponent)
  (params (OverlappedComponent :type Primitive%20Component%20Object%20Reference) (OtherActor :type Actor%20Object%20Reference) (OtherComp :type Primitive%20Component%20Object%20Reference) (OtherBodyIndex :type Integer) (bFromSweep :type Boolean) (SweepResult :type Hit%20Result%20Structure%20%28by%20ref%29))
  ;[0.1958 0.2839 1] CollisionToPlayer
  (if (Utilities|DoesObjectImplementInterface OtherActor "/Game/Interfaces/BPI_Damageable.BPI_Damageable_C")
    (Class|BPIDamageable|TakeDamage(Message) OtherActor (Variables|Default|GetDamageToPlayer))))

(event EventGetNuked
  (bind _playerref (Variables|Default|GetPlayerRef))
  ;[1 0.06262 0.294] EnemyIsNuked
  (bind _output_get (Variables|/Game/FirstPerson/Blueprints/BP_FirstPersonCharacter.BP_FirstPersonCharacter_C|SetEnemyDestroy _playerref (Variables|/Game/FirstPerson/Blueprints/BP_FirstPersonCharacter.BP_FirstPersonCharacter_C|GetEnemyDestroy _playerref)))
  (Math|Integer|IncrementInt _output_get
    (:%20%20
      (Actor|DestroyActor)
      (Default|EnemyDestroy (Variables|Default|GetWaveManagerREF)))))

(event EventBeginPlay
  ;[0.3829 1 0.2746] EnemyHP
  (Variables|Default|SetcurrentHP (Variables|Default|GetMaxHP))
  ;[0.2825 0.6912 1] Get a ref to player
  (bind _returnvalue (Actor|GetActorOfClass "/Game/FirstPerson/Blueprints/BP_FirstPersonCharacter.BP_FirstPersonCharacter_C"))
  (Variables|Default|SetPlayerRef _returnvalue)
  ;[0.4062 1 0.7861] Wave manager ref
  (bind _returnvalue_2 (Actor|GetActorOfClass "/Game/BP_WaveManager.BP_WaveManager_C"))
  (bind _output_get (Variables|Default|SetWaveManagerREF _returnvalue_2)))

(event EventTakeDamage
  (params (DamageTaken :type Integer))
  (bind _playerref (Variables|Default|GetPlayerRef))
  ;[1 0.2154 0.2851] Damage
  (bind _output_get (Variables|Default|SetcurrentHP (- (Variables|Default|GetcurrentHP) DamageTaken)))
  (bind _returnvalue (Actor|GetActorOfClass "/Game/BP_WaveManager.BP_WaveManager_C"))
  (if (<= _output_get 0)
    (Variables|/Game/BP_WaveManager.BP_WaveManager_C|SetEnemies%20alive _returnvalue (- (Variables|/Game/BP_WaveManager.BP_WaveManager_C|GetEnemies%20alive _returnvalue) 1))
    (Default|EnemyDestroy (stale EventBeginPlay _output_get))
    (bind _output_get_2 (Variables|/Game/FirstPerson/Blueprints/BP_FirstPersonCharacter.BP_FirstPersonCharacter_C|SetEnemyDestroy _playerref (Variables|/Game/FirstPerson/Blueprints/BP_FirstPersonCharacter.BP_FirstPersonCharacter_C|GetEnemyDestroy _playerref)))
    (Math|Integer|IncrementInt _output_get_2
      (:%20%20
        (Actor|DestroyActor)))))

(event EventTick
  (params (DeltaSeconds :type Float%20%28single-precision%29))
  ;[1 0.307 0.8549] Pathfinding
  (bind _returnvalue (Actor|GetActorOfClass "/Game/FirstPerson/Blueprints/BP_FirstPersonCharacter.BP_FirstPersonCharacter_C"))
  (AI|AIMoveTo self "0, 0, 0" _returnvalue 5.0 false))

(fn ConstructionScript)