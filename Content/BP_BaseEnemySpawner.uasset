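; Enemy spawner actor that periodically populates the area around itself with BP_BaseEnemy actors.
; A looping three-second timer, started on BeginPlay, spawns each enemy at a random reachable navigation point within Radius of the spawner.
; EnemyCount increments per spawn and is never decremented here, so spawning stops for good once it exceeds MaxEnemyCount.
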(event Custom|SpawnEnemy
  (if (<= (Variables|Default|GetEnemyCount) (Variables|Default|GetMaxEnemyCount))
    (Game|SpawnActorfromClass "/Game/BP_BaseEnemy.BP_BaseEnemy_C" (Math|Transform|MakeTransform (.RandomLocation (AI|Navigation|GetRandomReachablePointinRadius (Transformation|GetActorLocation) (Variables|Default|GetRadius) 0 0)) "0, 0, 0" "1.000000,1.000000,1.000000") "Undefined" "MultiplyWithRoot" 0 0)
    (Variables|Default|SetEnemyCount (+ (Variables|Default|GetEnemyCount) 1))))

(event EventBeginPlay
  (Utilities|Time|SetTimerbyEvent (delegate Custom|SpawnEnemy) 3.0 true))

(fn ConstructionScript)