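; Spawner actor that creates BP_RangeEnemy enemies at random reachable navmesh points within a radius of itself.
; The Spawnable event loops from EnemyCount to the requested number, with a latent Delay inside the loop body before the spawn.
; Spawning increments EnemiesAlive on BP_WaveManager, which is looked up again there rather than through the reference cached at BeginPlay.
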(event EventSpawnable
  (params (Enemy :type Integer))
  ;[0.3176 0.2314 1] Make enemies spawn
  (for _index (range (Variables|Default|GetEnemyCount) Enemy)
    (Utilities|FlowControl|Delay 2.0)
    (Game|SpawnActorfromClass "/Game/BP_RangeEnemy.BP_RangeEnemy_C" (Math|Transform|MakeTransform (.RandomLocation (AI|Navigation|GetRandomReachablePointinRadius (Transformation|GetActorLocation) (Variables|Default|GetRadius) 0 0)) "0, 0, 0" "1.000000,1.000000,1.000000") "Undefined" "MultiplyWithRoot" 0 0)
    (bind _returnvalue (Actor|GetActorOfClass "/Game/BP_WaveManager.BP_WaveManager_C"))
    (bind _result (Math|Integer|IncrementInt (Variables|/Game/BP_WaveManager.BP_WaveManager_C|GetEnemies%20alive _returnvalue))
      (:%20%20
        (Variables|/Game/BP_WaveManager.BP_WaveManager_C|SetEnemies%20alive _returnvalue _result)))))

(event EventBeginPlay
  ;[1 0.8648 0.5718] WaveManagerRef
  (bind _returnvalue (Actor|GetActorOfClass "/Game/BP_WaveManager.BP_WaveManager_C"))
  (Variables|Default|SetSpawnManagerREF _returnvalue))

(fn ConstructionScript)